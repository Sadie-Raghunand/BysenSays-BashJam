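; BP_BSAIController is an AI controller for the wood-chopping game that takes control of a player pawn.
; On possess it checks for a valid pawn, printing an error otherwise, then runs InitValues.
; InitValues caches the wood chop gamemode found in the level and the possessed BP_WoodChopGamePlayer, then flags that player as AI-possessed.
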(event EventBeginPlay)

(event EventTick
  (params (DeltaSeconds :type Float%20%28single-precision%29)))

(event EventPossess
  (params (PossessedPawn :type Pawn%20Object%20Reference))
  ;[0.15 0.15 0.15 0.5] Checking for valid player
  (Utilities|IsValid (Pawn|GetControlledPawn)
    (:Is%20Valid
      (CallFunction|InitValues))
    (:Is%20Not%20Valid
      (Development|PrintString "Invalid controlled pawn!" true true "(R=1.000000,G=0.000000,B=0.718364,A=1.000000)" 3e+01))))

(fn ConstructionScript)

(fn InitValues
  ;[0.15 0.15 0.15 0.5] Gamemode
  (bind _returnvalue (Actor|GetActorOfClass "/Game/Blueprints/BP_WoodChopGamemode.BP_WoodChopGamemode_C"))
  (Variables|Default|SetGamemode _returnvalue)
  ;[0.15 0.15 0.15 0.5] Player
  (bind _asbp_wood_chop_game_player (Utilities|Casting|CastToBP_WoodChopGamePlayer (Pawn|GetControlledPawn)))
  (bind _output_get (Variables|Default|SetPossessedPlayer _asbp_wood_chop_game_player))
  (Variables|/Game/Blueprints/BP_WoodChopGamePlayer.BP_WoodChopGamePlayer_C|SetIsAIPossessed _output_get true))