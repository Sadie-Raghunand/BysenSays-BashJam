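; Player actor for the rhythm wood-chop minigame, playable by a human or AI, that registers with BP_WoodChopGamemode.
; During listening measures, three chop-type inputs, gated by cooldown and per-bar beat count, are timed against the nearest beat.
; Human chops score on type match and timing offset, while AI rolls against success-rate intervals and derives animation delay from the score.
; Results drive team points, axe animations, rating text and empty-beat material flicker.
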(event Custom|FlickerPlayer
  ;[0 0 0 1 50] Visual/audio/UI cues
  ;;[0.15 0.15 0.15 0.5] Visual flicker feedback
  (for _index (range 0 4)
    (bind _output_get (Variables|Default|SetPlayerMat (Rendering|Material|GetMaterial (Variables|Default|GetSkeletalMesh) 0)))
    (Math|Integer|CompareInt (Math|Integer|%(Integer) _index 2)
      (:>
        (Rendering|Material|SetMaterial (Variables|Default|GetSkeletalMesh) 0 _output_get))
      (:==
        (Rendering|Material|SetMaterial (Variables|Default|GetSkeletalMesh) 0 "/BashAssets/Serenity/SharedMaterials/Wood/M_Wood.M_Wood")))
    (Utilities|FlowControl|Delay 0.05))
  (Rendering|Material|SetMaterial (Variables|Default|GetSkeletalMesh) 0 _output_get)
  (Utilities|FlowControl|Delay 0.05))

(event Custom|Event_CheckPlayerChops
  (bind _gamemode (Variables|Default|GetGamemode))
  ;[0.1055 0 0.15 0.5 100] OCCURS ON INPUT
  ;;[0 0 0 1 50] Scoring
  ;;;[1 0.255 0] Scoring assistance
  (bind (_beatval _haschop _beatidx) (Default|HelperCalcBeatVal _gamemode 0 true))
  (CallFunction|CheckifMissBeat (Variables|/Game/Blueprints/BP_WoodChopGamemode.BP_WoodChopGamemode_C|GetIsListening _gamemode) _haschop _beatidx))

(event Custom|ResetBeatsThisRepeat
  ;[0 0 0 1 50] Game reset/begining of gamesetup
  ;;[0.15 0.15 0.15 0.5] Reset after bar, called after gnome's measures
  (Variables|Default|SetBeatsThisRepeat 0)
  (Variables|Default|SetCurrentBarOfRepeat (+ (Variables|Default|GetCurrentBarOfRepeat) 1)))

(event Custom|Event_PlayAnimationOnChop
  (params (Pts :type Integer))
  ;[0 0 0 1 50] Visual/audio/UI cues
  ;;[0.7083 0.6124 0] Control timing of player animations, AI specific?
  (if (Variables|Default|GetIsAIPossessed) ; If normal player, don't artificially add delay, ai players, add delay
    (Utilities|FlowControl|Delay (Variables|Default|GetAIChopDelay))
    (CallFunction|PlayAxeChopAnim (> Pts 0))
    (else
      (CallFunction|PlayAxeChopAnim (> Pts 0))))
  (CallFunction|DisplaySuccessText Pts))

(event Input|EnhancedActionEvents|EnhancedInputActionIA_MediumFlex
  (params (ActionValue :type Boolean) (ElapsedSeconds :type Float%20%28double-precision%29) (TriggeredSeconds :type Float%20%28double-precision%29) (InputAction :type Input%20Action%20Object%20Reference :default "/LimbitlessBluetoothPlugin/InputActions/IA_MediumFlex.IA_MediumFlex"))
  (bind _gamemode (Variables|Default|GetGamemode))
  (bind _playernumber (Variables|Default|GetPlayerNumber))
  (bind _gamemode_2 (Variables|Default|GetGamemode))
  (bind _basepointcounter (Variables|/Game/Blueprints/BP_WoodChopGamemode.BP_WoodChopGamemode_C|GetBasePointCounter _gamemode))
  ;[0.1055 0 0.15 0.5 100] OCCURS ON INPUT
  ;;[0 0.001429 0.15 0.5 50] Input
  ;;;[0.15 0.15 0.15 0.5] Button type 2
  (:Started
    (Variables|Default|SetPlayerChopType 2)
    (if (Variables|/Game/Blueprints/BP_WoodChopGamemode.BP_WoodChopGamemode_C|GetIsListening (Variables|Default|GetGamemode)) ; Prevent input on gnome's measure
      (Variables|Default|SethasChoppedThisBeat true)
      (|DoOnceMultiInput
        (:A%20Out
          ;;[0.15 0.15 0.15 0.5] Calculate beat timing
          (Variables|Default|SetCooldownTime (Variables|Default|GetCooldownReset))
          (|++BeatsThisRepeat)
          (bind _output_get (Variables|Default|SetPlayerFlexTime (Utilities|Time|GetTimeSeconds)))
          (Math|Float|CompareFloat (|TimeFromLastBeat _gamemode_2 _output_get) (|TimeUntilNextBeat _gamemode_2 _output_get)
            (:>
              (bind _output_get_2 (Variables|Default|SetPlayerHitOffset (|TimeUntilNextBeat _gamemode_2 _output_get) :!label _label)) ; Use next beat
              (if (> (Variables|/Game/Blueprints/BP_WoodChopGamemode.BP_WoodChopGamemode_C|GetNextBeatVal (Variables|Default|GetGamemode)) 0) ; Check if the next beat is not empty
                ;;[0 0 0 1 50] Scoring
                ;;;[0.15 0.15 0.15 0.5] Scoring and UI feedbaclk
                (bind _points (CallFunction|AwardPointsforChop _output_get_2 (Variables|Default|GetPlayerChopType) (Variables|/Game/Blueprints/BP_WoodChopGamemode.BP_WoodChopGamemode_C|GetTmp_idx (Variables|Default|GetGamemode))))
                (CallFunction|EventPlayAnimationonChop _points)
                (Class|BasePointCounter|AddPoints _basepointcounter _playernumber _points)
                (Variables|Default|SetPlayerChopType 0 :!label _label_2) ; Reset chop
                (else
                  (CallFunction|EventPlayAnimationonChop)
                  (Utilities|Time|SetTimerbyEvent (delegate Custom|FlickerPlayer) 0.0 :!label _label_3))))
            (:==
              (goto _label))
            (:<
              (bind _output_get_3 (Variables|Default|SetPlayerHitOffset (|TimeFromLastBeat _gamemode_2 _output_get))) ; Use previous beat
              (if (> (Variables|/Game/Blueprints/BP_WoodChopGamemode.BP_WoodChopGamemode_C|GetLastBeatVal (Variables|Default|GetGamemode)) 0) ; Check if the last beat was not empty
                (bind _points_2 (CallFunction|AwardPointsforChop _output_get_3 (Variables|Default|GetPlayerChopType) (Variables|/Game/Blueprints/BP_WoodChopGamemode.BP_WoodChopGamemode_C|GetTmp_idx (Variables|Default|GetGamemode))))
                (CallFunction|EventPlayAnimationonChop _points_2)
                (Class|BasePointCounter|AddPoints _basepointcounter _playernumber _points_2)
                (goto _label_2)
                (else
                  (CallFunction|EventPlayAnimationonChop) ; Player chops where  there is no chop
                  (goto _label_3))))))))))

(event Input|EnhancedActionEvents|EnhancedInputActionIA_Button1
  (params (ActionValue :type Boolean) (ElapsedSeconds :type Float%20%28double-precision%29) (TriggeredSeconds :type Float%20%28double-precision%29) (InputAction :type Input%20Action%20Object%20Reference :default "/MinigameCore/Input/IA_Button1.IA_Button1"))
  (bind _gamemode (Variables|Default|GetGamemode))
  (bind _playernumber (Variables|Default|GetPlayerNumber))
  (bind _gamemode_2 (Variables|Default|GetGamemode))
  (bind _basepointcounter (Variables|/Game/Blueprints/BP_WoodChopGamemode.BP_WoodChopGamemode_C|GetBasePointCounter _gamemode))
  ;[0.1055 0 0.15 0.5 100] OCCURS ON INPUT
  ;;[0 0.001429 0.15 0.5 50] Input
  ;;;[0.15 0.15 0.15 0.5] Button type 1
  (:Started
    (Variables|Default|SetPlayerChopType 1)
    (if (Variables|/Game/Blueprints/BP_WoodChopGamemode.BP_WoodChopGamemode_C|GetIsListening (Variables|Default|GetGamemode)) ; Prevent input on gnome's measure
      (Variables|Default|SethasChoppedThisBeat true)
      (|DoOnceMultiInput
        (:A%20Out
          ;;[0.15 0.15 0.15 0.5] Calculate beat timing
          (Variables|Default|SetCooldownTime (Variables|Default|GetCooldownReset))
          (|++BeatsThisRepeat)
          (bind _output_get (Variables|Default|SetPlayerFlexTime (Utilities|Time|GetTimeSeconds)))
          (Math|Float|CompareFloat (|TimeFromLastBeat _gamemode_2 _output_get) (|TimeUntilNextBeat _gamemode_2 _output_get)
            (:>
              (bind _output_get_2 (Variables|Default|SetPlayerHitOffset (|TimeUntilNextBeat _gamemode_2 _output_get) :!label _label)) ; Use next beat
              (if (> (Variables|/Game/Blueprints/BP_WoodChopGamemode.BP_WoodChopGamemode_C|GetNextBeatVal (Variables|Default|GetGamemode)) 0) ; Check if the next beat is not empty
                ;;[0 0 0 1 50] Scoring
                ;;;[0.15 0.15 0.15 0.5] Scoring and UI feedbaclk
                (bind _points (CallFunction|AwardPointsforChop _output_get_2 (Variables|Default|GetPlayerChopType) (Variables|/Game/Blueprints/BP_WoodChopGamemode.BP_WoodChopGamemode_C|GetTmp_idx (Variables|Default|GetGamemode))))
                (CallFunction|EventPlayAnimationonChop _points)
                (Class|BasePointCounter|AddPoints _basepointcounter _playernumber _points)
                (Variables|Default|SetPlayerChopType 0 :!label _label_2) ; Reset chop
                (else
                  (CallFunction|EventPlayAnimationonChop)
                  (Utilities|Time|SetTimerbyEvent (delegate Custom|FlickerPlayer) 0.0 :!label _label_3))))
            (:==
              (goto _label))
            (:<
              (bind _output_get_3 (Variables|Default|SetPlayerHitOffset (|TimeFromLastBeat _gamemode_2 _output_get))) ; Use previous beat
              (if (> (Variables|/Game/Blueprints/BP_WoodChopGamemode.BP_WoodChopGamemode_C|GetLastBeatVal (Variables|Default|GetGamemode)) 0) ; Check if the last beat was not empty
                (bind _points_2 (CallFunction|AwardPointsforChop _output_get_3 (Variables|Default|GetPlayerChopType) (Variables|/Game/Blueprints/BP_WoodChopGamemode.BP_WoodChopGamemode_C|GetTmp_idx (Variables|Default|GetGamemode))))
                (CallFunction|EventPlayAnimationonChop _points_2)
                (Class|BasePointCounter|AddPoints _basepointcounter _playernumber _points_2)
                (goto _label_2)
                (else
                  (CallFunction|EventPlayAnimationonChop) ; Player chops where  there is no chop
                  (goto _label_3))))))))))

(event Input|EnhancedActionEvents|EnhancedInputActionIA_LightFlex
  (params (ActionValue :type Boolean) (ElapsedSeconds :type Float%20%28double-precision%29) (TriggeredSeconds :type Float%20%28double-precision%29) (InputAction :type Input%20Action%20Object%20Reference :default "/LimbitlessBluetoothPlugin/InputActions/IA_LightFlex.IA_LightFlex"))
  (bind _gamemode (Variables|Default|GetGamemode))
  (bind _playernumber (Variables|Default|GetPlayerNumber))
  (bind _gamemode_2 (Variables|Default|GetGamemode))
  (bind _basepointcounter (Variables|/Game/Blueprints/BP_WoodChopGamemode.BP_WoodChopGamemode_C|GetBasePointCounter _gamemode))
  ;[0.1055 0 0.15 0.5 100] OCCURS ON INPUT
  ;;[0 0.001429 0.15 0.5 50] Input
  ;;;[0.15 0.15 0.15 0.5] Button type 1
  (:Started
    (Variables|Default|SetPlayerChopType 1)
    (if (Variables|/Game/Blueprints/BP_WoodChopGamemode.BP_WoodChopGamemode_C|GetIsListening (Variables|Default|GetGamemode)) ; Prevent input on gnome's measure
      (Variables|Default|SethasChoppedThisBeat true)
      (|DoOnceMultiInput
        (:A%20Out
          ;;[0.15 0.15 0.15 0.5] Calculate beat timing
          (Variables|Default|SetCooldownTime (Variables|Default|GetCooldownReset))
          (|++BeatsThisRepeat)
          (bind _output_get (Variables|Default|SetPlayerFlexTime (Utilities|Time|GetTimeSeconds)))
          (Math|Float|CompareFloat (|TimeFromLastBeat _gamemode_2 _output_get) (|TimeUntilNextBeat _gamemode_2 _output_get)
            (:>
              (bind _output_get_2 (Variables|Default|SetPlayerHitOffset (|TimeUntilNextBeat _gamemode_2 _output_get) :!label _label)) ; Use next beat
              (if (> (Variables|/Game/Blueprints/BP_WoodChopGamemode.BP_WoodChopGamemode_C|GetNextBeatVal (Variables|Default|GetGamemode)) 0) ; Check if the next beat is not empty
                ;;[0 0 0 1 50] Scoring
                ;;;[0.15 0.15 0.15 0.5] Scoring and UI feedbaclk
                (bind _points (CallFunction|AwardPointsforChop _output_get_2 (Variables|Default|GetPlayerChopType) (Variables|/Game/Blueprints/BP_WoodChopGamemode.BP_WoodChopGamemode_C|GetTmp_idx (Variables|Default|GetGamemode))))
                (CallFunction|EventPlayAnimationonChop _points)
                (Class|BasePointCounter|AddPoints _basepointcounter _playernumber _points)
                (Variables|Default|SetPlayerChopType 0 :!label _label_2) ; Reset chop
                (else
                  (CallFunction|EventPlayAnimationonChop)
                  (Utilities|Time|SetTimerbyEvent (delegate Custom|FlickerPlayer) 0.0 :!label _label_3))))
            (:==
              (goto _label))
            (:<
              (bind _output_get_3 (Variables|Default|SetPlayerHitOffset (|TimeFromLastBeat _gamemode_2 _output_get))) ; Use previous beat
              (if (> (Variables|/Game/Blueprints/BP_WoodChopGamemode.BP_WoodChopGamemode_C|GetLastBeatVal (Variables|Default|GetGamemode)) 0) ; Check if the last beat was not empty
                (bind _points_2 (CallFunction|AwardPointsforChop _output_get_3 (Variables|Default|GetPlayerChopType) (Variables|/Game/Blueprints/BP_WoodChopGamemode.BP_WoodChopGamemode_C|GetTmp_idx (Variables|Default|GetGamemode))))
                (CallFunction|EventPlayAnimationonChop _points_2)
                (Class|BasePointCounter|AddPoints _basepointcounter _playernumber _points_2)
                (goto _label_2)
                (else
                  (CallFunction|EventPlayAnimationonChop) ; Player chops where  there is no chop
                  (goto _label_3))))))))))

(event Input|EnhancedActionEvents|EnhancedInputActionIA_StrongFlex
  (params (ActionValue :type Boolean) (ElapsedSeconds :type Float%20%28double-precision%29) (TriggeredSeconds :type Float%20%28double-precision%29) (InputAction :type Input%20Action%20Object%20Reference :default "/LimbitlessBluetoothPlugin/InputActions/IA_StrongFlex.IA_StrongFlex"))
  (bind _gamemode (Variables|Default|GetGamemode))
  (bind _playernumber (Variables|Default|GetPlayerNumber))
  (bind _gamemode_2 (Variables|Default|GetGamemode))
  (bind _basepointcounter (Variables|/Game/Blueprints/BP_WoodChopGamemode.BP_WoodChopGamemode_C|GetBasePointCounter _gamemode))
  ;[0.1055 0 0.15 0.5 100] OCCURS ON INPUT
  ;;[0 0.001429 0.15 0.5 50] Input
  ;;;[0.15 0.15 0.15 0.5] Beat type 3
  (:Started
    (Variables|Default|SetPlayerChopType 3)
    (if (Variables|/Game/Blueprints/BP_WoodChopGamemode.BP_WoodChopGamemode_C|GetIsListening (Variables|Default|GetGamemode)) ; Prevent input on gnome's measure
      (Variables|Default|SethasChoppedThisBeat true)
      (|DoOnceMultiInput
        (:A%20Out
          ;;[0.15 0.15 0.15 0.5] Calculate beat timing
          (Variables|Default|SetCooldownTime (Variables|Default|GetCooldownReset))
          (|++BeatsThisRepeat)
          (bind _output_get (Variables|Default|SetPlayerFlexTime (Utilities|Time|GetTimeSeconds)))
          (Math|Float|CompareFloat (|TimeFromLastBeat _gamemode_2 _output_get) (|TimeUntilNextBeat _gamemode_2 _output_get)
            (:>
              (bind _output_get_2 (Variables|Default|SetPlayerHitOffset (|TimeUntilNextBeat _gamemode_2 _output_get) :!label _label)) ; Use next beat
              (if (> (Variables|/Game/Blueprints/BP_WoodChopGamemode.BP_WoodChopGamemode_C|GetNextBeatVal (Variables|Default|GetGamemode)) 0) ; Check if the next beat is not empty
                ;;[0 0 0 1 50] Scoring
                ;;;[0.15 0.15 0.15 0.5] Scoring and UI feedbaclk
                (bind _points (CallFunction|AwardPointsforChop _output_get_2 (Variables|Default|GetPlayerChopType) (Variables|/Game/Blueprints/BP_WoodChopGamemode.BP_WoodChopGamemode_C|GetTmp_idx (Variables|Default|GetGamemode))))
                (CallFunction|EventPlayAnimationonChop _points)
                (Class|BasePointCounter|AddPoints _basepointcounter _playernumber _points)
                (Variables|Default|SetPlayerChopType 0 :!label _label_2) ; Reset chop
                (else
                  (CallFunction|EventPlayAnimationonChop)
                  (Utilities|Time|SetTimerbyEvent (delegate Custom|FlickerPlayer) 0.0 :!label _label_3))))
            (:==
              (goto _label))
            (:<
              (bind _output_get_3 (Variables|Default|SetPlayerHitOffset (|TimeFromLastBeat _gamemode_2 _output_get))) ; Use previous beat
              (if (> (Variables|/Game/Blueprints/BP_WoodChopGamemode.BP_WoodChopGamemode_C|GetLastBeatVal (Variables|Default|GetGamemode)) 0) ; Check if the last beat was not empty
                (bind _points_2 (CallFunction|AwardPointsforChop _output_get_3 (Variables|Default|GetPlayerChopType) (Variables|/Game/Blueprints/BP_WoodChopGamemode.BP_WoodChopGamemode_C|GetTmp_idx (Variables|Default|GetGamemode))))
                (CallFunction|EventPlayAnimationonChop _points_2)
                (Class|BasePointCounter|AddPoints _basepointcounter _playernumber _points_2)
                (goto _label_2)
                (else
                  (CallFunction|EventPlayAnimationonChop) ; Player chops where  there is no chop
                  (goto _label_3))))))))))

(event Input|EnhancedActionEvents|EnhancedInputActionIA_Button2
  (params (ActionValue :type Boolean) (ElapsedSeconds :type Float%20%28double-precision%29) (TriggeredSeconds :type Float%20%28double-precision%29) (InputAction :type Input%20Action%20Object%20Reference :default "/MinigameCore/Input/IA_Button2.IA_Button2"))
  (bind _gamemode (Variables|Default|GetGamemode))
  (bind _playernumber (Variables|Default|GetPlayerNumber))
  (bind _gamemode_2 (Variables|Default|GetGamemode))
  (bind _basepointcounter (Variables|/Game/Blueprints/BP_WoodChopGamemode.BP_WoodChopGamemode_C|GetBasePointCounter _gamemode))
  ;[0.1055 0 0.15 0.5 100] OCCURS ON INPUT
  ;;[0 0.001429 0.15 0.5 50] Input
  ;;;[0.15 0.15 0.15 0.5] Button type 2
  (:Started
    (Variables|Default|SetPlayerChopType 2)
    (if (Variables|/Game/Blueprints/BP_WoodChopGamemode.BP_WoodChopGamemode_C|GetIsListening (Variables|Default|GetGamemode)) ; Prevent input on gnome's measure
      (Variables|Default|SethasChoppedThisBeat true)
      (|DoOnceMultiInput
        (:A%20Out
          ;;[0.15 0.15 0.15 0.5] Calculate beat timing
          (Variables|Default|SetCooldownTime (Variables|Default|GetCooldownReset))
          (|++BeatsThisRepeat)
          (bind _output_get (Variables|Default|SetPlayerFlexTime (Utilities|Time|GetTimeSeconds)))
          (Math|Float|CompareFloat (|TimeFromLastBeat _gamemode_2 _output_get) (|TimeUntilNextBeat _gamemode_2 _output_get)
            (:>
              (bind _output_get_2 (Variables|Default|SetPlayerHitOffset (|TimeUntilNextBeat _gamemode_2 _output_get) :!label _label)) ; Use next beat
              (if (> (Variables|/Game/Blueprints/BP_WoodChopGamemode.BP_WoodChopGamemode_C|GetNextBeatVal (Variables|Default|GetGamemode)) 0) ; Check if the next beat is not empty
                ;;[0 0 0 1 50] Scoring
                ;;;[0.15 0.15 0.15 0.5] Scoring and UI feedbaclk
                (bind _points (CallFunction|AwardPointsforChop _output_get_2 (Variables|Default|GetPlayerChopType) (Variables|/Game/Blueprints/BP_WoodChopGamemode.BP_WoodChopGamemode_C|GetTmp_idx (Variables|Default|GetGamemode))))
                (CallFunction|EventPlayAnimationonChop _points)
                (Class|BasePointCounter|AddPoints _basepointcounter _playernumber _points)
                (Variables|Default|SetPlayerChopType 0 :!label _label_2) ; Reset chop
                (else
                  (CallFunction|EventPlayAnimationonChop)
                  (Utilities|Time|SetTimerbyEvent (delegate Custom|FlickerPlayer) 0.0 :!label _label_3))))
            (:==
              (goto _label))
            (:<
              (bind _output_get_3 (Variables|Default|SetPlayerHitOffset (|TimeFromLastBeat _gamemode_2 _output_get))) ; Use previous beat
              (if (> (Variables|/Game/Blueprints/BP_WoodChopGamemode.BP_WoodChopGamemode_C|GetLastBeatVal (Variables|Default|GetGamemode)) 0) ; Check if the last beat was not empty
                (bind _points_2 (CallFunction|AwardPointsforChop _output_get_3 (Variables|Default|GetPlayerChopType) (Variables|/Game/Blueprints/BP_WoodChopGamemode.BP_WoodChopGamemode_C|GetTmp_idx (Variables|Default|GetGamemode))))
                (CallFunction|EventPlayAnimationonChop _points_2)
                (Class|BasePointCounter|AddPoints _basepointcounter _playernumber _points_2)
                (goto _label_2)
                (else
                  (CallFunction|EventPlayAnimationonChop) ; Player chops where  there is no chop
                  (goto _label_3))))))))))

(event Input|EnhancedActionEvents|EnhancedInputActionIA_Button3
  (params (ActionValue :type Boolean) (ElapsedSeconds :type Float%20%28double-precision%29) (TriggeredSeconds :type Float%20%28double-precision%29) (InputAction :type Input%20Action%20Object%20Reference :default "/MinigameCore/Input/IA_Button3.IA_Button3"))
  (bind _gamemode (Variables|Default|GetGamemode))
  (bind _playernumber (Variables|Default|GetPlayerNumber))
  (bind _gamemode_2 (Variables|Default|GetGamemode))
  (bind _basepointcounter (Variables|/Game/Blueprints/BP_WoodChopGamemode.BP_WoodChopGamemode_C|GetBasePointCounter _gamemode))
  ;[0.1055 0 0.15 0.5 100] OCCURS ON INPUT
  ;;[0 0.001429 0.15 0.5 50] Input
  ;;;[0.15 0.15 0.15 0.5] Beat type 3
  (:Started
    (Variables|Default|SetPlayerChopType 3)
    (if (Variables|/Game/Blueprints/BP_WoodChopGamemode.BP_WoodChopGamemode_C|GetIsListening (Variables|Default|GetGamemode)) ; Prevent input on gnome's measure
      (Variables|Default|SethasChoppedThisBeat true)
      (|DoOnceMultiInput
        (:A%20Out
          ;;[0.15 0.15 0.15 0.5] Calculate beat timing
          (Variables|Default|SetCooldownTime (Variables|Default|GetCooldownReset))
          (|++BeatsThisRepeat)
          (bind _output_get (Variables|Default|SetPlayerFlexTime (Utilities|Time|GetTimeSeconds)))
          (Math|Float|CompareFloat (|TimeFromLastBeat _gamemode_2 _output_get) (|TimeUntilNextBeat _gamemode_2 _output_get)
            (:>
              (bind _output_get_2 (Variables|Default|SetPlayerHitOffset (|TimeUntilNextBeat _gamemode_2 _output_get) :!label _label)) ; Use next beat
              (if (> (Variables|/Game/Blueprints/BP_WoodChopGamemode.BP_WoodChopGamemode_C|GetNextBeatVal (Variables|Default|GetGamemode)) 0) ; Check if the next beat is not empty
                ;;[0 0 0 1 50] Scoring
                ;;;[0.15 0.15 0.15 0.5] Scoring and UI feedbaclk
                (bind _points (CallFunction|AwardPointsforChop _output_get_2 (Variables|Default|GetPlayerChopType) (Variables|/Game/Blueprints/BP_WoodChopGamemode.BP_WoodChopGamemode_C|GetTmp_idx (Variables|Default|GetGamemode))))
                (CallFunction|EventPlayAnimationonChop _points)
                (Class|BasePointCounter|AddPoints _basepointcounter _playernumber _points)
                (Variables|Default|SetPlayerChopType 0 :!label _label_2) ; Reset chop
                (else
                  (CallFunction|EventPlayAnimationonChop)
                  (Utilities|Time|SetTimerbyEvent (delegate Custom|FlickerPlayer) 0.0 :!label _label_3))))
            (:==
              (goto _label))
            (:<
              (bind _output_get_3 (Variables|Default|SetPlayerHitOffset (|TimeFromLastBeat _gamemode_2 _output_get))) ; Use previous beat
              (if (> (Variables|/Game/Blueprints/BP_WoodChopGamemode.BP_WoodChopGamemode_C|GetLastBeatVal (Variables|Default|GetGamemode)) 0) ; Check if the last beat was not empty
                (bind _points_2 (CallFunction|AwardPointsforChop _output_get_3 (Variables|Default|GetPlayerChopType) (Variables|/Game/Blueprints/BP_WoodChopGamemode.BP_WoodChopGamemode_C|GetTmp_idx (Variables|Default|GetGamemode))))
                (CallFunction|EventPlayAnimationonChop _points_2)
                (Class|BasePointCounter|AddPoints _basepointcounter _playernumber _points_2)
                (goto _label_2)
                (else
                  (CallFunction|EventPlayAnimationonChop) ; Player chops where  there is no chop
                  (goto _label_3))))))))))

(event EventOnReset
  ;[0 0 0 1 50] Game reset/begining of gamesetup
  ;;[0.15 0.15 0.15 0.5] Game reset after finished
  (Variables|Default|SetCurrentBarOfRepeat 0)
  (Variables|Default|SetBeatsThisRepeat 0))

(event EventTick
  (params (DeltaSeconds :type Float%20%28single-precision%29))
  (bind _gamemode (Variables|Default|GetGamemode))
  (bind _playernumber (Variables|Default|GetPlayerNumber))
  (bind _gamemode_2 (Variables|Default|GetGamemode))
  (bind _basepointcounter (Variables|/Game/Blueprints/BP_WoodChopGamemode.BP_WoodChopGamemode_C|GetBasePointCounter _gamemode))
  ;[0.1055 0 0.15 0.5 100] OCCURS ON INPUT
  ;;[0 0.001429 0.15 0.5 50] Input
  ;;;[0.15 0.15 0.15 0.5] Keep player input within their own beats
  (Math|Float|CompareFloat (Variables|Default|GetCooldownTime) 0.0
    (:>
      (Variables|Default|SetCooldownTime (- (Variables|Default|GetCooldownTime) DeltaSeconds)))
    (:==
      (Math|Integer|CompareInt (Variables|Default|GetBeatsThisRepeat) (Utilities|Array|Get(acopy) (Variables|Default|GetBeatsInRepeat) (Variables|Default|GetCurrentBarOfRepeat)) :!label _label ; First player measure, never gpes past 0 beats this repeat?
        (:<
          (|DoOnceMultiInput) ; enters at Reset In
        )))
    (:<
      (goto _label))))

(event EventBeginPlay
  ;[0 0 0 1 50] Game reset/begining of gamesetup
  ;;[0.03801 0.8594 0] Begin minigame
  (bind _asbp_wood_chop_gamemode (Utilities|Casting|CastToBP_WoodChopGamemode (Game|GetGameMode)))
  (bind _output_get (Variables|Default|SetGamemode _asbp_wood_chop_gamemode))
  (EventDispatchers|BindEventtoOnRepeatBarChange _output_get (delegate Custom|ResetBeatsThisRepeat))
  (Variables|Default|SetBeatsThisRepeat 0)
  (Variables|Default|SetCurrentBarOfRepeat 0)
  (Components|Animation|PlayAnimation (Variables|Default|GetSkeletalMesh) "/BashAssets/Character/Modular/Animations/AN_ModCharaIdle.AN_ModCharaIdle" true) ; IDLE
  (Utilities|Array|Add (Variables|/Game/Blueprints/BP_WoodChopGamemode.BP_WoodChopGamemode_C|GetWoodchopPlayers (Variables|Default|GetGamemode)) self))

(event Input|KeyboardEvents|DebugKeyB
  (params (Key :type Key%20Structure :default "None") (ActionValue :type Input%20Action%20Value%20Structure))
  ;[0.15 0 0 0.5 50] Debugging
  (:Pressed
    (Class|MinigameBase|EndGame (Variables|Default|GetGamemode))))

(fn ConstructionScript)

(fn AwardPointsforChop
  (params (HitOffset :type Float%20%28double-precision%29) (PlayerChopType :type Integer) (BeatIndex :type Integer))
  (if (Variables|Default|GetIsAIPossessed)
    ;[0 0.001429 0.9913 0.5] AI players
    (bind _pointstoaward (CallFunction|AIChopBehvaior))
    (CallFunction|DisplaySuccessText _pointstoaward)
    (return _pointstoaward)
    (else
      ;[0.03801 0.8594 0 0.2609] Player - new
      ;;[0 0 0] Check if  player did correct type of chop, if yes then award 5 pts base before additional calculations
      (bind _beatval (Default|HelperCalcBeatVal (Variables|Default|GetGamemode) (- BeatIndex 4) false))
      (if (== _beatval PlayerChopType)
        (LocalVariables|SetPts 5.0)
        (if (> HitOffset 1.0) ; Split offset into two, greater and less than 1
          ;;[0 0 0 0.5] Point calculation based on hit offset
          ;;;[0.2812 0.002741 0 1 14] Deduct points, further from beat
          (if (> HitOffset 1.5) ; Split again, 1-2
            (LocalVariables|SetPts (- (LocalVariables|GetPts) 3.0))
            (else
              (LocalVariables|SetPts (- (LocalVariables|GetPts) 1.0))))
          (else
            ;;;[0 1 0 0.5 14] Add Points, very close/exact on beat
            (if (> HitOffset 0.5) ; Split again, 0-0.99
              (LocalVariables|SetPts (+ (LocalVariables|GetPts) 3.0))
              (else
                (LocalVariables|SetPts (+ (LocalVariables|GetPts) 5.0))))))
        (return (Math|Float|Truncate (LocalVariables|GetPts)))
        (else
          (return 0) ; Return no points for the wrong beat type
        )))))

(fn DisplaySuccessText
  (params (PointNum :type Integer))
  (bind _asbp_success_message (Utilities|Casting|CastToBP_SuccessMessage (UserInterface|GetWidget (Variables|Default|GetSuccessMessage))))
  (switch int PointNum
    (:0
      (CallFunction|DisplayMiss) ; Fail, no points
    )
    (:1
      (bind _output_get (Variables|Default|SetCurrSuccessText "OKAY!" :!label _label))
      (bind _output_get_2 (Variables|Default|SetCurrSuccessColor "(R=0.610496,G=0.039546,B=0.024158,A=1.000000)"))
      (Default|SetWordText _asbp_success_message _output_get _output_get_2))
    (:2
      (goto _label))
    (:3
      (goto _label))
    (:4
      (goto _label))
    (:5
      (bind _output_get_3 (Variables|Default|SetCurrSuccessText "GOOD!" :!label _label_2))
      (bind _output_get_4 (Variables|Default|SetCurrSuccessColor "(R=0.991102,G=0.376262,B=0.040915,A=1.000000)"))
      (Default|SetWordText _asbp_success_message _output_get_3 _output_get_4))
    (:6
      (goto _label_2))
    (:7
      (bind _output_get_5 (Variables|Default|SetCurrSuccessText "AWESOME!" :!label _label_3))
      (bind _output_get_6 (Variables|Default|SetCurrSuccessColor "(R=0.258183,G=0.539479,B=0.068478,A=1.000000)"))
      (Default|SetWordText _asbp_success_message _output_get_5 _output_get_6))
    (:8
      (goto _label_3))
    (:9
      (bind _output_get_7 (Variables|Default|SetCurrSuccessText "PERFECT!" :!label _label_4))
      (bind _output_get_8 (Variables|Default|SetCurrSuccessColor "(R=0.064803,G=0.080220,B=0.479320,A=1.000000)"))
      (Default|SetWordText _asbp_success_message _output_get_7 _output_get_8))
    (:10
      (goto _label_4))))

(fn DisplayMiss
  (bind _output_get (Variables|Default|SetCurrSuccessText "MISS!"))
  (bind _output_get_2 (Variables|Default|SetCurrSuccessColor "(R=0.661458,G=0.148972,B=0.093018,A=1.000000)"))
  (bind _asbp_success_message (Utilities|Casting|CastToBP_SuccessMessage (UserInterface|GetWidget (Variables|Default|GetSuccessMessage))))
  (Default|SetWordText _asbp_success_message _output_get _output_get_2))

(fn CheckifMissBeat
  (params (isListening :type Boolean) (hasChop :type Boolean) (TMP_CheckAgainst :type Integer))
  (if isListening ; True if player's turn, check if the beat is 0 and player provides no input but there was supposed to be input, show success/fail text
    (if hasChop
      (if (Variables|Default|GethasChoppedThisBeat)
        (CallFunction|DisplayMiss)))))

(fn SetBeatsinRepeat
  (params (Index :type Integer) (NumBeats :type Integer))
  (Utilities|Array|SetArrayElem (Variables|Default|GetBeatsInRepeat) Index NumBeats))

(fn AIChopBehvaior
  (bind _rateofsuccess (LocalVariables|GetRateOfSuccess))
  (bind _gamemode (Variables|Default|GetGamemode))
  ;[0 0 0 0.5] Housekeeping to get the correct beat for this beat, set an array with incorrect beats to pick
  (bind _beatval (Default|HelperCalcBeatVal _gamemode (- (Variables|/Game/Blueprints/BP_WoodChopGamemode.BP_WoodChopGamemode_C|GetTmp_idx _gamemode) 3) false))
  (bind _output_get (LocalVariables|SetCorrectBeat _beatval))
  (Utilities|Array|RemoveItem (LocalVariables|GetIncorrectChopSets) _output_get)
  ;[0.15 0.15 0.15 0.5] Generate random int to compare against success rate
  (LocalVariables|SetGeneratedVal (Math|Random|RandomIntegerinRange 0 100))
  ;[1 1 1 0.5] Check score intervals
  (bind (_array_element _array_index) (Utilities|Array|ForEachLoopwithBreak _rateofsuccess) ; Iterate through intervals of scores/offsets
    (:LoopBody
      ;[0.008682 1 0] Value is in this scoring interval, set score and return
      (if (Math|Float|InRange(Float) (Math|Conversions|ToFloat(Integer) (LocalVariables|GetGeneratedVal)) (Utilities|Array|Get(acopy) _rateofsuccess (+ _array_index 1)) _array_element)
        (Variables|Default|SetPlayerChopType (LocalVariables|GetCorrectBeat))
        (Class|BasePointCounter|AddPoints (Variables|/Game/Blueprints/BP_WoodChopGamemode.BP_WoodChopGamemode_C|GetBasePointCounter (Variables|Default|GetGamemode)) (Variables|Default|GetTeam) (Utilities|Array|Get(acopy) (LocalVariables|GetIntervalsOfScores) _array_index))
        (bind _delay (CallFunction|AIChopAnimDelayCalc (- 1.0 (* (Utilities|Array|Get(acopy) (LocalVariables|GetIntervalsOfScores) _array_index) 0.1)) (Utilities|Array|Get(acopy) (LocalVariables|GetIntervalsOfScores) _array_index)))
        (Variables|Default|SetAIChopDelay _delay)
        (CallFunction|EventPlayAnimationonChop (Utilities|Array|Get(acopy) (LocalVariables|GetIntervalsOfScores) _array_index))
        (return (Utilities|Array|Get(acopy) (LocalVariables|GetIntervalsOfScores) _array_index))))
    (:Completed
      ;[1 0.01173 0] Incorrect beat type, 0 pts
      (Variables|Default|SetPlayerChopType (Math|Random|RandomIntegerinRange 0 (- (Utilities|Array|Length (LocalVariables|GetIncorrectChopSets)) 1)))
      (Class|BasePointCounter|AddPoints (Variables|/Game/Blueprints/BP_WoodChopGamemode.BP_WoodChopGamemode_C|GetBasePointCounter (Variables|Default|GetGamemode)) (Variables|Default|GetTeam))
      (CallFunction|EventPlayAnimationonChop)
      (return 0))))

(fn PlayAxeChopAnim
  (params (Hit :type Boolean))
  (if Hit
    (Components|Animation|PlayAnimation (Variables|Default|GetSkeletalMesh) "/Game/Gnome/AM_ModChara_AxeHit.AM_ModChara_AxeHit" false) ; HIT
    (Components|Animation|PlayAnimation (Variables|Default|GetAxeSkel) "/Game/Axe/Animations/SK_Gnome_Axe_Hit.SK_Gnome_Axe_Hit" false)
    (else
      (Components|Animation|PlayAnimation (Variables|Default|GetSkeletalMesh) "/Game/AxeModCharaAnimations/ModChara_AxeMiss.ModChara_AxeMiss" false) ; MISS
      (Components|Animation|PlayAnimation (Variables|Default|GetAxeSkel) "/Game/Axe/Animations/SK_Gnome_Axe_Miss.SK_Gnome_Axe_Miss" false))))

(fn AIChopAnimDelayCalc
  (params (PercentOffset :type Float%20%28double-precision%29) (Pts :type Integer))
  (if (Math|Integer|InRange(Integer) Pts 1 6)
    (LocalVariables|SetDelayVal (* 2.4 PercentOffset))
    (bind _output_get (LocalVariables|SetLate (Math|Random|RandomBool)))
    (if _output_get
      _
      (else
        (LocalVariables|SetDelayVal (* (LocalVariables|GetDelayVal) -1.0))))
    (bind _output_get_2 (LocalVariables|SetDelayVal (+ 2.4 (LocalVariables|GetDelayVal))))
    (return (/ _output_get_2 4.0))
    (else
      (return (/ (LocalVariables|GetDelayVal) 4.0)) ; On time
    )))

(fn StopAI
  (if (Variables|Default|GetIsAIPossessed)
    (Variables|Default|SetIsAIPossessed false)))