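; Game mode for a wood-chopping rhythm minigame where players listen to a gnome's chop pattern, then repeat it.
; A Quartz clock starts quantized music and drives bar and beat events that advance the pattern, trigger AI chops, flag misses and end the game.
; An 80-beat randomized chop array alternates listen and repeat measures, feeding turn-prompt and chop-type UI.
; It also handles "Get Ready" pauses, spawn placement, practice resets and tie-aware winner names.
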(event Custom|OnBeat
  (params (ClockName :type Name) (QuantizationType :type EQuartzCommandQuantization%20Enum :default "Bar") (NumBars :type Integer) (Beat :type Integer) (BeatFraction :type Float%20%28single-precision%29))
  (Development|PrintString (Utilities|String|ToString(Integer) (Variables|Default|GetIdx)) true true (.SpecifiedColor (Utilities|Struct|BreakSlateColor (Variables|Default|GetCurrentListeningColor))))
  ;[0.1055 0 0.15 0.5 60] BEAT
  (bind _alreadyfired (CallFunction|CalcTimeSinceFire (Variables|Default|GetLastBeatTime)))
  (if (not _alreadyfired)
    (for _array_element (Variables|Default|GetWoodchopPlayers)
      ;;[0.15 0.15 0.15 0.5] Handle AI behavior each beat, IN LOOP
      (Utilities|IsValid _array_element ; Prevent null errors bw resets in practice
        (:Is%20Valid
          (if (Variables|/Game/Blueprints/BP_WoodChopGamePlayer.BP_WoodChopGamePlayer_C|GetIsAIPossessed _array_element)
            (if (Variables|Default|GetIsListening)
              (if (not (Math|Integer|InRange(Integer) (Variables|Default|GetChopIndex) 0 4)) ; :D access none error in actual game, not practice
                (Default|AIChopBehvaior _array_element)))))))
    (if (Variables|Default|GetinCutscene) ; Exit loop
      (if (Variables|Default|GetbIsPractice)
        ;;[0.15 0.15 0.15 0.5] Reset chop? Check timing/order of execution on this
        (for _array_element_2 (Class|MinigameBase|GetPlayers) :!label _label
          ;;[0 0.1615 0.159 0.5] Looped
          (bind _asbp_wood_chop_game_player (Utilities|Casting|CastToBP_WoodChopGamePlayer _array_element_2))
          (Default|EventCheckPlayerChops _asbp_wood_chop_game_player)
          (bind _haschop (CallFunction|HelperCalcBeatVal (- Beat 0) false))
          (if (not _haschop)
            (if (Variables|/Game/Blueprints/BP_WoodChopGamePlayer.BP_WoodChopGamePlayer_C|GethasChoppedThisBeat _asbp_wood_chop_game_player)
              (Variables|/Game/Blueprints/BP_WoodChopGamePlayer.BP_WoodChopGamePlayer_C|SethasChoppedThisBeat _asbp_wood_chop_game_player false)
              (Default|DisplayMiss _asbp_wood_chop_game_player) ; Note for debugging: Recently swapped positions with se has chopped this beat in case that breaks anyhing!
            )))
        (|IsMeaureUnpaused
          (:then
            (Development|PrintString "Hello")
            (Default|CallUpdateChopUI true) ; Repeat
          )
          (:else
            _))
        ;;[0.15 0.15 0.15 0.5] Get last beat, next beat's projected time, and which measure beat is on
        (Variables|Default|SetTimeAtLastBeat (Utilities|Time|GetTimeSeconds))
        (Variables|Default|SetTimeAtNextBeat (+ (Variables|Default|GetTimeAtLastBeat) 0.6))
        (Variables|Default|SetCurrBeatOfMeasure (+ (Variables|Default|GetCurrBeatOfMeasure) 1))
        (if (|GetChopBeatsatChopIndex)
          (Default|CallOnBeatHasChop)
          (Default|CallUpdateChopTypeUI false) ; Don't clear
        )
        (bind _output_get (Variables|Default|SetChopIndex (+ (Variables|Default|GetChopIndex) 1)))
        (Math|Integer|CompareInt (- _output_get 4)
          (:>
            (bind _beatval (CallFunction|HelperCalcBeatVal (- _output_get 4) false :!label _label_2))
            (Variables|Default|SetLastBeatVal _beatval))
          (:==
            (goto _label_2))
          (:<
            (Variables|Default|SetLastBeatVal 0)))
        (Math|Integer|CompareInt (- (Variables|Default|GetChopIndex) 4)
          (:>
            ;;[0 0 0 0.5] Go to next beat
            (bind _beatval_2 (CallFunction|HelperCalcBeatVal (- (Variables|Default|GetChopIndex) 4) false :!label _label_3))
            (Variables|Default|SetNextBeatVal _beatval_2))
          (:==
            (goto _label_3))
          (:<
            (Variables|Default|SetNextBeatVal 0))))
      (else
        (goto _label)))))

(event Custom|StartClockEvent
  (params (EventType :type EQuartzCommandDelegateSubType%20Enum :default "CommandOnFailedToQueue") (Name :type Name))
  (switch Utilities|FlowControl|Switch|SwitchonEQuartzCommandDelegateSubType EventType
    (:CommandOnQueued
      (bind _clockhandle (Class|QuartzClockHandle|StartClock (Variables|Default|GetMainClock))) ; everything here only happens on queuw
      (bind _clockhandle_2 (Class|QuartzClockHandle|SubscribetoQuantizationEvent _clockhandle "Beat" (delegate Custom|OnBeat)))
      (Class|QuartzClockHandle|SubscribetoQuantizationEvent _clockhandle_2 "Bar" (delegate Custom|OnBar)))))

(event Custom|OnGameReset_Event
  ;[1 0 0.03805] Begining of game these occur, include all event bindings for events that do not run at begining of game
  ;;[0.15 0.15 0.15 0.5] Setup
  (Default|CallUpdateChopTypeUI true)
  (Variables|Default|SetBegining true)
  (Variables|Default|SetCurrentListeningText "Listen then repeat!")
  (Variables|Default|SetCurrentListeningColor (Utilities|Struct|MakeSlateColor "(R=1.000000,G=0.964643,B=0.830429,A=1.000000)"))
  (CallFunction|SetBeatswithChops)
  (Variables|Default|SetIsListening true)
  (Variables|Default|SetinBetweenTurns false))

(event Custom|ResetClock
  ;[0.5811 0.1928 1] Occurs every time the clock gets reset, when game resets (enter play mode, loop in practice)
  (CallFunction|GameResetInit (delegate Custom|ResetStartClock)))

(event Custom|Event_PauseBeats
  ;[0.15 0.15 0.15 0.5] Allow for pause bw gnome and player measures, at begining of event, should show get ready, at end show repeate, at end of repeat switch to listen
  (Development|PrintString "¯\\_(ツ)_/¯" true true "(R=1.000000,G=0.788855,B=0.179731,A=1.000000)")
  (Variables|Default|SetinBetweenTurns true)
  (Class|QuartzClockHandle|PauseClock (Variables|Default|GetMainClock)) ; Right after this, clock returns as running for one beat,\n then after that false, but remains on same beat\nThis happens while listen text is up (probably bc the ui call is after this)
  (Class|AudioComponent|SetPaused (Variables|Default|GetMusicComponent) true)
  (Utilities|FlowControl|Delay 2.0)
  (Class|QuartzClockHandle|ResumeClock (Variables|Default|GetMainClock))
  (Class|AudioComponent|SetPaused (Variables|Default|GetMusicComponent) false)
  (Default|CallUpdateChopUI true))

(event Custom|Event_GamePlayStart
  (Variables|Default|SetinCutscene false) ; Previously connected to set beats  w chops
  ;[1 0 0.03805 1 35] Begin play
  (bind _returnvalue (Audio|SpawnSound2D (Variables|Default|GetMusic) 1.0 1.0 0.0 0))
  (bind _output_get (Variables|Default|SetMusicComponent _returnvalue))
  (if (Variables|Default|GetbIsPractice)
    (Audio|Components|Audio|PlayQuantized _returnvalue (Variables|Default|GetMainClock) (Utilities|Struct|MakeQuartzQuantizationBoundary "Beat" 1.0 "TransportRelative") (delegate Custom|StartClockEvent)) ; Starts all quantization events
    (elif (Variables|Default|GetinCutscene)
      (Class|QuartzClockHandle|StopClock (Variables|Default|GetMainClock) true))))

(event Custom|OnBar
  (params (ClockName :type Name) (QuantizationType :type EQuartzCommandQuantization%20Enum :default "Bar") (NumBars :type Integer) (Beat :type Integer) (BeatFraction :type Float%20%28single-precision%29))
  ;[0.15 0 0.05579 0.5 60] BAR
  (Development|PrintString (Utilities|String|ToString(Integer) (Variables|Default|GetIdx)))
  (if (Variables|Default|GetinCutscene)
    (if (Variables|Default|GetbIsPractice)
      (Math|Integer|CompareInt NumBars 1 :!label _label ; Check song has started
        (:>
          (Math|Integer|CompareInt NumBars 20
            (:>
              (Class|MinigameBase|EndGame :!label _label_2)
              (Default|CallGameEndUI) ; If reached 20 bars, end game, end of song
            )
            (:==
              (goto _label_2))
            (:<
              ;;[0.15 0.15 0.15 0.5] This occurs on listen + get ready, not repeate
              (Default|CallUpdateChopUI false) ; Flip UI called here "listen"\n\nn%8=0 && n%8=4\n\nCalled on bar
              (Variables|Default|SetCurrBeatOfMeasure 1)
              (Math|Integer|CompareInt NumBars 3
                (:>
                  _)
                (:==
                  _))
              (Math|Integer|CompareInt (Math|Integer|%(Integer) NumBars 2)
                (:>
                  _)
                (:<
                  _))
              (Default|CallOnRepeatBarChange))))))
    (else
      (goto _label))))

(event Custom|ResetStartClock
  (params (EventType :type EQuartzCommandDelegateSubType%20Enum :default "CommandOnFailedToQueue") (Name :type Name))
  ;[0.5811 0.1928 1] Occurs every time the clock gets reset, when game resets (enter play mode, loop in practice)
  (switch Utilities|FlowControl|Switch|SwitchonEQuartzCommandDelegateSubType EventType
    (:CommandOnQueued
      ;;[0.15 0.15 0.15 0.5] Restart clock
      (Class|QuartzClockHandle|StartClock (Variables|Default|GetMainClock)))))

(event EventTick
  (params (DeltaSeconds :type Float%20%28single-precision%29))
  (Variables|Default|SetTimeBwBeats DeltaSeconds))

(event EventOnMinigameStart
  ;[1 0 0.03805] Begining of game these occur, include all event bindings for events that do not run at begining of game
  ;;[0.15 0.15 0.15 0.5] When game starts, randomize beats/chops
  (CallFunction|FindSpawns) ; For ensuring player is in correct position\nThere must be a better solution for this
  (if (Variables|Default|GetbIsPractice)
    (CallFunction|SetBeatswithChops)
    ;[1 0 0.03805 1 35] Begin play
    (Variables|Default|SetCurrentListeningText "Listen then repeat!")
    (Variables|Default|SetCurrentListeningColor (Utilities|Struct|MakeSlateColor "(R=1.000000,G=0.964643,B=0.830429,A=1.000000)"))
    (EventDispatchers|BindEventtoOnMinigameResetEvent (delegate Custom|ResetClock))
    (|CallParentFunction)
    (Variables|Default|SetPointCounter (Class|MinigameBase|GetPointCounter))
    (bind _returnvalue (Class|QuartzSubsystem|CreateNewClock (WorldSubsystems|GetQuartzSubsystem) "MainClock" (Utilities|Struct|MakeQuartzClockSettings (Utilities|Struct|MakeQuartzTimeSignature 4 "QuarterNote") false) false))
    (bind _clockhandle (Class|QuartzClockHandle|SetBeatsPerMinute _returnvalue (Utilities|Struct|MakeQuartzQuantizationBoundary "Beat" 1.0 "TransportRelative") 0 (Variables|Default|GetDefaultBPM)))
    (Variables|Default|SetMainClock _clockhandle)
    (bind _returnvalue_2 (Audio|SpawnSound2D (Variables|Default|GetMusic) 1.0 1.0 0.0 0))
    (bind _output_get (Variables|Default|SetMusicComponent _returnvalue_2))
    (if (Variables|Default|GetbIsPractice)
      (Audio|Components|Audio|PlayQuantized _returnvalue_2 (Variables|Default|GetMainClock) (Utilities|Struct|MakeQuartzQuantizationBoundary "Beat" 1.0 "TransportRelative") (delegate Custom|StartClockEvent)) ; Starts all quantization events
      (elif (Variables|Default|GetinCutscene)
        (Class|QuartzClockHandle|StopClock (Variables|Default|GetMainClock) true)))))

(event EventOnMinigameEnd
  ;[0.15 0.1078 0.02138 0.5 50] Check end game
  (for _array_element (Variables|Default|GetWoodchopPlayers)
    (Utilities|IsValid _array_element
      (:Is%20Valid
        (Default|StopAI _array_element)))))

(fn ConstructionScript
  (|CallParentFunction))

(fn FlipUI
  (params (JustPaused :type Boolean))
  (bind _idx (Variables|Default|GetIdx))
  (bind _returnvalue (Math|Integer|%(Integer) _idx 8))
  ;[0.15 0.15 0.15 0.5] Avoid starting cycle during cutscene
  (Variables|Default|SetBegining false)
  (if (Variables|Default|GetinCutscene)
    (if (Variables|Default|GetbIsPractice)
      ;[0.3883 1 0] The big Refactor *TM
      (Development|PrintString (Utilities|String|ToString(Integer) _returnvalue) true true "(R=0.000000,G=0.000000,B=0.000000,A=1.000000)")
      (if (.IsGnomeBeat (Utilities|Struct|BreakE_BeatData (Utilities|Array|Get(acopy) (Variables|Default|GetChopBeatData) (Variables|Default|GetIdx)))) ; True - listen\nFalse - repeat
        ;[0.15 0.15 0.15 0.5] Gnome turn
        (bind _output_get (Variables|Default|SetCurrentListeningText "Listen!"))
        (bind _output_get_2 (Variables|Default|SetCurrentListeningColor (Utilities|Struct|MakeSlateColor "(R=0.000000,G=0.174952,B=0.859375,A=1.000000)")))
        (Variables|Default|SetIsListening false) ; Change to GNOME turn
        (elif (== _returnvalue 0)
          ;[0.15 0.15 0.15 0.5] Player turn
          (Variables|Default|SetinBetweenTurns false :!label _label) ; Check for true on this bc switch from get ready to repeat,\n\nset false here bc that state is no longer in place
          (bind _output_get_3 (Variables|Default|SetCurrentListeningText "Repeat!"))
          (bind _output_get_4 (Variables|Default|SetCurrentListeningColor (Utilities|Struct|MakeSlateColor "(R=0.038006,G=0.859375,B=0.000000,A=1.000000)")))
          (Variables|Default|SetIsListening true) ; Change to PLAYER turn
          (Development|PrintString (Utilities|String|Append ":((((   " (Utilities|String|ToString(Integer) (Variables|Default|GetIdx))) true true "(R=1.000000,G=0.018091,B=0.000000,A=1.000000)")
          (elif JustPaused
            (goto _label)
            (else
              (Development|PrintString (Utilities|String|Append ":))))   " (Utilities|String|ToString(Integer) 0)) true true "(R=0.122632,G=1.000000,B=0.000000,A=1.000000)")
              ;[0.15 0.15 0.15 0.5] Between turns, how to get this to run on beats w/remainder 7?  This should run once every round, then the subsequent call should go to the repeat section
              (Default|CallUpdateChopTypeUI true) ; CLEAR type text temporarily
              (CallFunction|EventPauseBeats) ; n%8 = 0
              (bind _output_get_5 (Variables|Default|SetCurrentListeningText "Get Ready!"))
              (bind _output_get_6 (Variables|Default|SetCurrentListeningColor (Utilities|Struct|MakeSlateColor "(R=0.355240,G=0.859375,B=0.367349,A=1.000000)")))))))
      ;[1 0.2719 0 0.5] Debugging - show measure on text object to make more obvioujs, nnot permanent
      (bind _output_get_7 (Variables|Default|SetCurrentListeningText (Utilities|Text|ToText(String) (Utilities|String|Append (Utilities|String|ToString(Text) (Variables|Default|GetCurrentListeningText)) " " (Utilities|String|ToString(Integer) (Variables|Default|GetIdx))))))
      (return (Variables|Default|GetCurrentListeningColor) _output_get_7))))

(fn GetReadyUI
  (bind _output_get (Variables|Default|SetCurrentListeningText "GET READY!"))
  (bind _output_get_2 (Variables|Default|SetCurrentListeningColor (Utilities|Struct|MakeSlateColor "(R=0.661458,G=0.058844,B=0.019338,A=1.000000)")))
  (return _output_get_2 _output_get))

(fn ChopTypeUI
  (params (Clear :type Boolean))
  (if Clear
    ;[0.05969 0.15 0.06286 0.5] Clear text after listen measure
    (Variables|Default|SetChopTypeText "") ; Clear text after gnome turn
    (return (Utilities|Struct|MakeSlateColor "(R=1.000000,G=0.000000,B=1.000000,A=1.000000)") "")
    (else
      (bind (_beatval _haschop _beatidx) (CallFunction|HelperCalcBeatVal (- (Variables|Default|GetIdx) 1) false))
      ;[0.15 0 0.08619 0.5] Set text
      (if _haschop
        (Variables|Default|SetChopTypeText (Utilities|Text|ToText(String) (Utilities|String|Append (Utilities|String|ToString(Integer) _beatidx) " idx " (Utilities|String|ToString(Integer) (Variables|Default|GetIdx)))))
        (else
          (Variables|Default|SetChopTypeText "")))
      ;[0 0.001429 0.15 0.5] Set text color
      (switch int _beatval
        (:0
          _)
        (:1
          (Variables|Default|SetChopTypeUIColor (Utilities|Struct|MakeSlateColor "(R=0.171885,G=0.177899,B=1.000000,A=1.000000)")))
        (:2
          (Variables|Default|SetChopTypeUIColor (Utilities|Struct|MakeSlateColor "(R=1.000000,G=0.344483,B=0.512656,A=1.000000)")))
        (:3
          (Variables|Default|SetChopTypeUIColor (Utilities|Struct|MakeSlateColor "(R=1.000000,G=0.877768,B=0.198563,A=1.000000)"))))
      (return (Variables|Default|GetChopTypeUIColor) (Utilities|Text|ToText(String) (Utilities|String|Append (Utilities|String|ToString(Text) (Variables|Default|GetChopTypeText)) " " (Utilities|String|ToString(Integer) (Variables|Default|GetIdx))))))))

(fn GoodJobUI
  (bind _output_get (Variables|Default|SetCurrentListeningText "GOOD JOB!"))
  (bind _output_get_2 (Variables|Default|SetCurrentListeningColor (Utilities|Struct|MakeSlateColor "(R=0.258183,G=0.539479,B=0.068478,A=1.000000)")))
  (return _output_get_2 _output_get))

(fn SetBeatswithChops
  ;[0 0 0 0.5] Resize array to fit all beats, iterate to set all
  (Utilities|Array|Resize (Variables|Default|GetChopBeatData) 80)
  (for (_ _array_index) (Variables|Default|GetChopBeatData)
    (LocalVariables|Setindex _array_index)
    (if (== (LocalVariables|GetBeatTracker) 4) ; Check if at end of meausre
      ;[0.15 0.06016 0.06016 0.5 25] Behavior on last beat of the measure - this should run only once every 4 measures
      (if (LocalVariables|GetListenMeasure) ; If listen measure, set chops, else no chops
        ;;[0 0 0] there is a chop on this beat, set value
        (Utilities|Array|SetArrayElem (Variables|Default|GetChopBeatData) (LocalVariables|Getindex) (Utilities|Struct|MakeE_BeatData true (Math|Random|RandomIntegerinRange 1 3) true))
        (elif (< (LocalVariables|GetChopsInMeasure) (LocalVariables|GetMinNumCPM)) ; If not enough chops in meausre, set this beat to a chop
          (Utilities|Array|SetArrayElem (Variables|Default|GetChopBeatData) (LocalVariables|Getindex) (Utilities|Struct|MakeE_BeatData false 0 false) :!label _label)
          (elif (Math|Random|RandomBool) ; If has chops, randomize chop on this beat
            (goto _label)
            (else
              ;;[0 0 0 0.5] No chop this beat
              (Utilities|Array|SetArrayElem (Variables|Default|GetChopBeatData) (LocalVariables|Getindex) (Utilities|Struct|MakeE_BeatData false 0 false))))))
      (for _array_element (Class|MinigameBase|GetPlayers) ; Ierate through players
        (bind _asbp_wood_chop_game_player (Utilities|Casting|CastToBP_WoodChopGamePlayer _array_element))
        (Default|SetBeatsinRepeat _asbp_wood_chop_game_player (LocalVariables|GetPlayerRepeatIndex) (+ (LocalVariables|GetChopsInMeasure) 1)) ; Set the number of beats that have chops in the current measure being set
      )
      ;[0.02917 0.15 0.02706 0.5] Reset for next measure
      (LocalVariables|SetBeatTracker 1) ; Handle reset beat tracker
      (LocalVariables|SetChopsInMeasure 0)
      (bind _output_get (LocalVariables|SetListenMeasure (not (LocalVariables|GetListenMeasure))))
      (if (not _output_get)
        (Math|Integer|IncrementInt (LocalVariables|GetPlayerRepeatIndex)))
      (else
        ;[0.5252 0.4391 0.776 0.5 25] NOT END ON MEAUSRE
        (if (LocalVariables|GetListenMeasure) ; If listen measure (gnome turn), set chops, else no chops
          (if (< (LocalVariables|GetChopsInMeasure) (LocalVariables|GetMaxNumCPM)) ; Check if at maximum number of chops per measure
            ;[0.15 0.15 0.15 0.5] Set the beat to have a chop or not randomly
            (if (Math|Random|RandomBool)
              (bind _output_get_2 (LocalVariables|SetTMP_BeatIdxCreate (Math|Random|RandomIntegerinRange 1 3)))
              (Utilities|Array|SetArrayElem (Variables|Default|GetChopBeatData) (LocalVariables|Getindex) (Utilities|Struct|MakeE_BeatData true _output_get_2 true))
              ;[0.1233 0.03528 0.15 0.5] Add a chop to counter if this beat has a chop on it
              (if (> (.BeatType (Utilities|Struct|BreakE_BeatData (Utilities|Array|Get(acopy) (Variables|Default|GetChopBeatData) (LocalVariables|Getindex)))) 0)
                (Math|Integer|IncrementInt (LocalVariables|GetChopsInMeasure)
                  (:%20%20
                    _)))
              (else
                (LocalVariables|SetTMP_BeatIdxCreate 0)))
            (else
              (LocalVariables|SetTMP_BeatIdxCreate 0)))
          (else
            ;;[0.15 0.15 0.15 0.5] No chop on this beat, not a listen/gnome measure
            (Utilities|Array|SetArrayElem (Variables|Default|GetChopBeatData) (LocalVariables|Getindex) (Utilities|Struct|MakeE_BeatData false 0 false))))
        ;[0.15 0.1119 0.03399 0.5] Move to next beat
        (Math|Integer|IncrementInt (LocalVariables|GetBeatTracker))))))

(fn HelperCalcBeatVal
  (params (Index :type Integer) (CheckLastMeasure :type Boolean))
  (if (== Index 0)
    ;[0.15 0.15 0.15 0.5] Makes index an optional parameter
    (if CheckLastMeasure
      (LocalVariables|SetProperIdx (- (Variables|Default|GetIdx) 4))
      (else
        (LocalVariables|SetProperIdx (Variables|Default|GetIdx))))
    (else
      (LocalVariables|SetProperIdx Index)))
  (if (> (.BeatType (Utilities|Struct|BreakE_BeatData (Utilities|Array|Get(acopy) (Variables|Default|GetChopBeatData) (LocalVariables|GetProperIdx)))) 0)
    (return (.BeatType (Utilities|Struct|BreakE_BeatData (Utilities|Array|Get(acopy) (Variables|Default|GetChopBeatData) (LocalVariables|GetProperIdx)))) true (LocalVariables|GetProperIdx) (Utilities|Array|Get(acopy) (Variables|Default|GetChopBeatData) (LocalVariables|GetProperIdx))) ; Return that the gnome chops on this beat
    (else
      (return (.BeatType (Utilities|Struct|BreakE_BeatData (Utilities|Array|Get(acopy) (Variables|Default|GetChopBeatData) (LocalVariables|GetProperIdx)))) false (LocalVariables|GetProperIdx) (Utilities|Array|Get(acopy) (Variables|Default|GetChopBeatData) (LocalVariables|GetProperIdx))) ; Return that the player chops on this beat
    )))

(fn ReturnWinnerName
  (bind _returnvalue (Class|GameModeBase|GetNumPlayers))
  ;[0.15 0.15 0.15 0.5] Iterate through points each player has, compare againts highest player score
  (for _index (range 0 _returnvalue)
    (if (> (Class|BasePointCounter|GetPointsbyPlayer (Variables|Default|GetBasePointCounter) _index) (LocalVariables|GetHighestScore)) ; Player has higher score, new high score
      (Utilities|Array|Resize (LocalVariables|GetWinnerTextSet) 1)
      ;[0.09727 0.5104 0.03167 0.5] Set high score players as part of array
      (Utilities|Array|SetArrayElem (LocalVariables|GetWinnerTextSet) 0 (Utilities|String|MakeLiteralString (Utilities|String|Append "Player " (Utilities|String|ToString(Integer) (+ _index 1)))))
      (LocalVariables|SetHighestScore (Class|BasePointCounter|GetPointsbyPlayer (Variables|Default|GetBasePointCounter) _index) :!label _label)
      (elif (== (Class|BasePointCounter|GetPointsbyPlayer (Variables|Default|GetBasePointCounter) _index) (LocalVariables|GetHighestScore)) ; High score players are tied, more than one winner possibly
        (Utilities|Array|Add (LocalVariables|GetWinnerTextSet) (Utilities|String|MakeLiteralString (Utilities|String|Append "Player " (Utilities|String|ToString(Integer) (+ _index 1)))))
        (goto _label))))
  ;[0.5081 0.3317 1 0.5] Return all winners' names as text for UI
  (return (LocalVariables|GetWinnerTextSet)))

(fn FindSpawns
  ;[0.15 0.15 0.15 0.5] Find spawns
  (bind _outactors (Actor|GetAllActorsOfClass "/MinigameCore/Game/BP_MinigamePlayerSpawn.BP_MinigamePlayerSpawn_C"))
  (Variables|Default|SetPlayerSpawns _outactors)
  ;[0.15 0.15 0.15 0.5] Get players and set rotations/locations
  (bind _outactors_2 (Actor|GetAllActorsOfClass "/Game/Blueprints/BP_WoodChopGamePlayer.BP_WoodChopGamePlayer_C"))
  (for (_array_element _array_index) _outactors_2
    (Transformation|SetActorLocationAndRotation _array_element (Transformation|GetActorLocation (Utilities|Array|Get(acopy) (Variables|Default|GetPlayerSpawns) _array_index)) "0.000000,-90.000000,0.000000")))

(fn CalcTimeSinceFire
  (params (Last%20beat%20time :type Float%20%28double-precision%29))
  (bind _returnvalue (Utilities|Time|GetGameTimeinSeconds))
  (if (< (- _returnvalue Last%20beat%20time) (Variables|Default|GetTimeBwBeats))
    (Variables|Default|SetLastBeatTime _returnvalue)
    (return true)
    (else
      (Variables|Default|SetLastBeatTime _returnvalue)
      (return false))))

(fn GameResetInit
  (params (InDelegate :type Delegate%20%28by%20ref%29))
  (Variables|Default|SetIdx 0)
  ;[0.15 0.15 0.15 0.5] Stop clock and reset time start/end time
  (Audio|Components|Audio|Stop (Variables|Default|GetMusicComponent))
  (bind _clockhandle (Class|QuartzClockHandle|StopClock (Variables|Default|GetMainClock) false))
  (Class|QuartzClockHandle|ResetTransport _clockhandle)
  ;[0.15 0.15 0.15 0.5] Reset sounds
  (bind _returnvalue (Audio|SpawnSound2D (Variables|Default|GetMusic) 1.0 1.0 0.0 0))
  (Variables|Default|SetMusicComponent _returnvalue)
  (Audio|Components|Audio|PlayQuantized _returnvalue _clockhandle (Utilities|Struct|MakeQuartzQuantizationBoundary "Beat" 1.0 "TransportRelative") InDelegate)
  ;[0.15 0.15 0.15 0.5] Clear player points
  (Variables|Default|SetChopIndex 0)
  (for (_ _array_index) (Variables|Default|GetPlayerObjects)
    (Class|BasePointCounter|SetPoints (Variables|Default|GetBasePointCounter) _array_index)))

(fn TMPPPPP
  (params (is%20clock%20running :type Boolean) (Extra :type String))
  (bind _debugprintcolors (Variables|Default|GetDebugPrintColors))
  (Development|PrintString (Utilities|String|Append "Set in between turns to true   " (Utilities|String|ToString(Integer) (Variables|Default|GetIdx)) (Utilities|String|ToString(Text) (Variables|Default|GetCurrentListeningText)) " - " (Utilities|String|ToString(Boolean) is%20clock%20running) Extra) true true (Math|Conversions|ToLinearColor(Color) (Utilities|Array|Get(acopy) _debugprintcolors (Math|Random|RandomIntegerinRange 0 (Utilities|Array|LastIndex _debugprintcolors))))))

(fn TestChangeUI
  (params (TextShouldSay :type Text) (TextColor :type Slate%20Color%20Structure) (ChangeIsListening :type Boolean))
  (Variables|Default|SetIsListening ChangeIsListening)
  (return TextColor TextShouldSay))